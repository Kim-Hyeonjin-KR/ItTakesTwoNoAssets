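; BP_DropableWall is a level actor wall that moves vertically when activated or deactivated and respawns players who touch its trigger box.
; OnActivate drives the mesh's height from its BeginPlay location with a timeline.
; OnDeActivate uses a second timeline to add relative Z offsets, then snaps the mesh back to that start location after a short delay.
; Box overlap calls Respawn on the overlapping character's BP_PlayerController, regardless of wall state.
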(event OnComponentBeginOverlap(Box)
  (params (OverlappedComponent :type Primitive%20Component%20Object%20Reference) (OtherActor :type Actor%20Object%20Reference) (OtherComp :type Primitive%20Component%20Object%20Reference) (OtherBodyIndex :type Integer) (bFromSweep :type Boolean) (SweepResult :type Hit%20Result%20Structure%20%28by%20ref%29))
  (bind _asit_takes_two_character (Utilities|Casting|CastToItTakesTwoCharacter OtherActor))
  (bind _asbp_player_controller (Utilities|Casting|CastToBP_PlayerController (Pawn|GetController _asit_takes_two_character)))
  (Default|Respawn _asbp_player_controller))

(event EventBeginPlay
  (Variables|Default|SetInitLocation (Transformation|GetWorldLocation (Variables|Default|GetStaticMesh))))

(event Collision|EventActorBeginOverlap
  (params (OtherActor :type Actor%20Object%20Reference)))

(event EventTick
  (params (DeltaSeconds :type Float%20%28single-precision%29)))

(event EventOnActivate
  (params (SelfActor :type Actor%20Object%20Reference))
  (bind _initlocation (Variables|Default|GetInitLocation))
  (bind _newtrack_0 (Timeline|Timeline_0 PlayFromStart)
    (:Update
      (Transformation|SetWorldLocation (Variables|Default|GetStaticMesh) (Math|Vector|MakeVector (.x _initlocation) (.y _initlocation) (+ (.z _initlocation) _newtrack_0)) false false))))

(event EventOnDeActivate
  (params (SelfActor :type Actor%20Object%20Reference))
  (bind _newlocationz (Timeline|Timeline PlayFromStart)
    (:Update
      (Transformation|AddRelativeLocation (Variables|Default|GetStaticMesh) (Math|Vector|MakeVector 0.0 0.0 _newlocationz) false false))
    (:Finished
      (Utilities|FlowControl|RetriggerableDelay 0.3)
      (Transformation|SetWorldLocation (Variables|Default|GetStaticMesh) (Variables|Default|GetInitLocation) false false))))

(fn ConstructionScript)