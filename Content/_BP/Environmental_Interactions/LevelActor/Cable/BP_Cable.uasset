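; BP_Cable is an activatable level cable that visually powers up along its mesh.
; BeginPlay creates a dynamic material on the cable and parks its MoveOffset parameter at the idle value.
; OnActivate animates MoveOffset with a timeline, then spawns a Niagara effect at the Box location.
; Deactivation is empty, and the timer-polled CheckActive shutoff is marked unused, its timer setup never running.
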(event Custom|CheckActive
  ;[1 1 1] 사용 안하는 기능
  (if (not (Variables|Default|GetbAllSwitchsActive))
    (Utilities|FlowControl|Sequence
      (:then_0
        (Development|PrintString "종료"))
      (:then_1
        (Utilities|Time|ClearandInvalidateTimerbyHandle (Variables|Default|GetTimerHandle)))
      (:then_2
        (bind _timevalue (Timeline|Timeline_0 PlayFromStart)
          (:Update
            (Rendering|Material|SetScalarParameterValue (Variables|Default|GetPowerLineMaterial) "MoveOffset" _timevalue :!class /Script/Engine.MaterialInstanceDynamic))
          (:Finished
            (Rendering|Material|SetScalarParameterValue (Variables|Default|GetPowerLineMaterial) "MoveOffset" -5.0 :!class /Script/Engine.MaterialInstanceDynamic)))))))

(event EventBeginPlay
  (bind _returnvalue (Rendering|Material|CreateDynamicMaterialInstance (Variables|Default|GetStaticMesh) 0 "/Game/_BP/Environmental_Interactions/LevelActor/Cable/Cords_01.Cords_01" "None" :!class /Script/Engine.PrimitiveComponent))
  (bind _output_get (Variables|Default|SetPowerLineMaterial _returnvalue))
  (Rendering|Material|SetScalarParameterValue _output_get "MoveOffset" -5.0 :!class /Script/Engine.MaterialInstanceDynamic))

(event EventTick
  (params (DeltaSeconds :type Float%20%28single-precision%29)))

(event EventOnActivate
  (params (SelfActor :type Actor%20Object%20Reference))
  (Utilities|FlowControl|Sequence
    (:then_0
      (bind _timevalue (Timeline|Timeline PlayFromStart)
        (:Update
          (Rendering|Material|SetScalarParameterValue (Variables|Default|GetPowerLineMaterial) "MoveOffset" _timevalue :!class /Script/Engine.MaterialInstanceDynamic))
        (:Finished
          (Niagara|SpawnSystematLocation "/Game/Basic_VFX/Niagara/NS_Basic_3.NS_Basic_3" (Transformation|GetWorldLocation (Variables|Default|GetBox))))))
    (:then_2
      (Development|PrintString "전선 활성화"))))

(event EventOnDeActivate
  (params (SelfActor :type Actor%20Object%20Reference)))

(fn ConstructionScript)