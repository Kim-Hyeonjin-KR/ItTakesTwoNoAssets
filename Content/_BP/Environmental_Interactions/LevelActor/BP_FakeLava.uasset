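; BP_FakeLava is a level actor that presents a toggleable lava surface, switching between an active orange state and an inactive blue state.
; On BeginPlay it creates a dynamic ember material on LavaMesh and starts active.
; ActiveLava and DeactiveLava toggle LavaCollision between query-only and disabled while recoloring the material's emission.
; The collision's begin-overlap event is empty, so the actor applies no effect on contact itself.
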(event OnComponentBeginOverlap(LavaCollision)
  (params (OverlappedComponent :type Primitive%20Component%20Object%20Reference) (OtherActor :type Actor%20Object%20Reference) (OtherComp :type Primitive%20Component%20Object%20Reference) (OtherBodyIndex :type Integer) (bFromSweep :type Boolean) (SweepResult :type Hit%20Result%20Structure%20%28by%20ref%29)))

(event Custom|DeactiveLava
  (Collision|SetCollisionEnabled (Variables|Default|GetLavaCollision) "NoCollision")
  (Rendering|Material|SetVectorParameterValue (Variables|Default|GetDynamicLavaMaterial) "Emission Color" "(R=0.000000,G=0.132107,B=1.000000,A=1.000000)" :!class /Script/Engine.MaterialInstanceDynamic))

(event Custom|ActiveLava
  (Collision|SetCollisionEnabled (Variables|Default|GetLavaCollision) "QueryOnly")
  (Rendering|Material|SetVectorParameterValue (Variables|Default|GetDynamicLavaMaterial) "Emission Color" "(R=1.000000,G=0.400000,B=0.000000,A=1.000000)" :!class /Script/Engine.MaterialInstanceDynamic))

(event EventBeginPlay
  (bind _returnvalue (Rendering|Material|CreateDynamicMaterialInstance (Variables|Default|GetLavaMesh) 0 "/Game/Fantastic_Village_Pack/materials/MI_ember_Inst.MI_ember_Inst" "None" :!class /Script/Engine.PrimitiveComponent))
  (Variables|Default|SetDynamicLavaMaterial _returnvalue)
  (CallFunction|ActiveLava))

(event Collision|EventActorBeginOverlap
  (params (OtherActor :type Actor%20Object%20Reference)))

(event EventTick
  (params (DeltaSeconds :type Float%20%28single-precision%29)))

(fn ConstructionScript)