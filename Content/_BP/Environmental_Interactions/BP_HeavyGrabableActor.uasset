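; Heavy grabbable environmental actor with an aura that neutralizes lava around it once the item is activated.
; ActiveItem turns on query-only collision for AuraCollision and prints a debug message.
; BP_Lava or BP_FakeLava actors entering the aura are deactivated through DeactiveLava, then reactivated through ActiveLava when the overlap ends.
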(event OnComponentBeginOverlap(AuraCollision)
  (params (OverlappedComponent :type Primitive%20Component%20Object%20Reference) (OtherActor :type Actor%20Object%20Reference) (OtherComp :type Primitive%20Component%20Object%20Reference) (OtherBodyIndex :type Integer) (bFromSweep :type Boolean) (SweepResult :type Hit%20Result%20Structure%20%28by%20ref%29))
  (bind _asbp_lava (Utilities|Casting|CastToBP_Lava OtherActor)
    (:then
      (Default|DeactiveLava _asbp_lava))
    (:CastFailed
      (bind _asbp_fake_lava (Utilities|Casting|CastToBP_FakeLava OtherActor))
      (Default|DeactiveLava _asbp_fake_lava))))

(event OnComponentEndOverlap(AuraCollision)
  (params (OverlappedComponent :type Primitive%20Component%20Object%20Reference) (OtherActor :type Actor%20Object%20Reference) (OtherComp :type Primitive%20Component%20Object%20Reference) (OtherBodyIndex :type Integer))
  (bind _asbp_lava (Utilities|Casting|CastToBP_Lava OtherActor)
    (:then
      (Default|ActiveLava _asbp_lava))
    (:CastFailed
      (bind _asbp_fake_lava (Utilities|Casting|CastToBP_FakeLava OtherActor))
      (Default|ActiveLava _asbp_fake_lava))))

(event EventBeginPlay)

(event Collision|EventActorBeginOverlap
  (params (OtherActor :type Actor%20Object%20Reference)))

(event EventTick
  (params (DeltaSeconds :type Float%20%28single-precision%29)))

(event EventActiveItem
  (Collision|SetCollisionEnabled (Variables|Default|GetAuraCollision) "QueryOnly")
  (Development|PrintString "아우라 활성화"))

(fn ConstructionScript)