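; Toggle lever interactable that tilts its handle when used and can be locked by an incoming signal.
; Interacting runs the parent interaction, then plays one of two timelines, chosen by HandleTiltLeft, to animate handle pitch.
; The first OnSignal sets Active, calls the parent interaction without animating the handle, then sets SignalLock to block further interaction and prints the state.
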(event Custom|SetHandleRotator
  (if (Variables|Default|GetbHandleTiltLeft)
    (bind _newrotatory (Timeline|Timeline_1 PlayFromStart)
      (:Update
        (Transformation|SetRelativeRotation (Variables|Default|GetLever_Handle) (Math|Rotator|MakeRotator 0.0 _newrotatory 0.0) false false)))
    (else
      (bind _newrotatory_2 (Timeline|Timeline PlayFromStart)
        (:Update
          (Transformation|SetRelativeRotation (Variables|Default|GetLever_Handle) (Math|Rotator|MakeRotator 0.0 _newrotatory_2 0.0) false false))))))

(event EventBeginPlay)

(event Collision|EventActorBeginOverlap
  (params (OtherActor :type Actor%20Object%20Reference)))

(event EventTick
  (params (DeltaSeconds :type Float%20%28single-precision%29)))

(event EventOnSignal
  (params (Interactor :type Actor%20Object%20Reference) (bSignal :type Boolean))
  (Utilities|FlowControl|DoOnce false
    (:Completed
      (Variables|Default|SetbActive true)
      (|CallParentFunction 0)
      (Variables|Default|SetbSignalLock true)
      (Development|PrintString (Utilities|String|ToString(Boolean) (Variables|Default|GetbActive))))))

(fn ConstructionScript)

(fn ActiveItemInteract
  (params (Interactor :type Actor%20Object%20Reference))
  (if (not (Variables|Default|GetbSignalLock))
    (bind _returnvalue (|CallParentFunction 0))
    (CallFunction|SetHandleRotator)
    (return _returnvalue)))