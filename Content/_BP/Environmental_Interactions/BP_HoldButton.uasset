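; BP_HoldButton is an interactable environmental button, with press and release feedback layered on a parent interaction class.
; Unless ActiveLock is set, activation calls the parent, then brightens the ButtonHandle material and nudges the handle inward along X.
; Deactivation calls the parent and reverses both changes without checking the lock.
; OnSignal only prints a Korean debug message announcing chain hold-button activation.
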(event EventBeginPlay)

(event Collision|EventActorBeginOverlap
  (params (OtherActor :type Actor%20Object%20Reference)))

(event EventTick
  (params (DeltaSeconds :type Float%20%28single-precision%29)))

(event EventDeactiveItemInteract
  (params (Interactor :type Actor%20Object%20Reference))
  (|CallParentFunction 0)
  (bind _button_handle (Variables|Default|GetButton_Handle)
    (:then
      (Rendering|Material|SetScalarParameterValueonMaterials _button_handle "Brightness" 1.0)
      (Transformation|SetRelativeLocation _button_handle (+ (Variables|/Script/Engine.SceneComponent|GetRelativeLocation _button_handle) "10.000000,0.000000,0.000000") false false))
    (:else)))

(event EventOnSignal
  (params (Interactor :type Actor%20Object%20Reference) (bSignal :type Boolean))
  (Development|PrintString "체인 홀드 버튼 활성화 "))

(fn ConstructionScript)

(fn ActiveItemInteract
  (params (Interactor :type Actor%20Object%20Reference))
  (if (not (LocalVariables|GetbActiveLock))
    (bind _returnvalue (|CallParentFunction 0))
    (bind _button_handle (Variables|Default|GetButton_Handle)
      (:then
        (Rendering|Material|SetScalarParameterValueonMaterials _button_handle "Brightness" 1e+01)
        (Transformation|SetRelativeLocation _button_handle (+ (Variables|/Script/Engine.SceneComponent|GetRelativeLocation _button_handle) "-10.000000,0.000000,0.000000") false false)
        (return _returnvalue))
      (:else))))