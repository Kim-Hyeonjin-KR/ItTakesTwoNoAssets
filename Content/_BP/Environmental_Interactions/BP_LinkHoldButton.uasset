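; Hold-button interactable that can only be pressed during a timed window opened by a signal.
; OnSignal waits through a retriggerable delay, then enables the button briefly, switching the handle's color between white and red.
; Interacting inside the window calls the parent logic, brightens the handle and pushes it in.
; Deactivating always calls the parent, dims the handle and shifts it back out, even if the press was rejected.
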(event Custom|DeActiveChainButton
  (Variables|Default|SetChainButtonActive false)
  (Development|PrintString "체인 엑티브 종료"))

(event EventBeginPlay)

(event Collision|EventActorBeginOverlap
  (params (OtherActor :type Actor%20Object%20Reference)))

(event EventTick
  (params (DeltaSeconds :type Float%20%28single-precision%29)))

(event EventDeactiveItemInteract
  (params (Interactor :type Actor%20Object%20Reference))
  (Variables|Default|SetCurrentInteract false)
  (|CallParentFunction 0)
  (bind _button_handle (Variables|Default|GetButton_Handle)
    (:then
      (Rendering|Material|SetScalarParameterValueonMaterials _button_handle "Brightness" 1.0)
      (Transformation|SetRelativeLocation _button_handle (+ (Variables|/Script/Engine.SceneComponent|GetRelativeLocation _button_handle) "10.000000,0.000000,0.000000") false false))
    (:else)))

(event EventOnSignal
  (params (Interactor :type Actor%20Object%20Reference) (bSignal :type Boolean))
  (Utilities|FlowControl|RetriggerableDelay 5.0)
  (Development|PrintString "5초가 지나서 홀드버튼 활성화")
  (Variables|Default|SetChainButtonActive true)
  (Rendering|Material|SetVectorParameterValueonMaterials (Variables|Default|GetButton_Handle) "ColorParam" "1.000000,1.000000,1.000000")
  (Utilities|FlowControl|RetriggerableDelay 2.0)
  (Variables|Default|SetChainButtonActive false)
  (Rendering|Material|SetVectorParameterValueonMaterials (Variables|Default|GetButton_Handle) "ColorParam" "1.000000,0.000000,0.000000")
  (Development|PrintString "그리고 2초가 지나서 홀드 버튼 비활성화"))

(fn ConstructionScript)

(fn ActiveItemInteract
  (params (Interactor :type Actor%20Object%20Reference))
  (Variables|Default|SetCurrentInteract true)
  (if (Variables|Default|GetChainButtonActive)
    (bind _returnvalue (|CallParentFunction 0))
    (bind _button_handle (Variables|Default|GetButton_Handle)
      (:then
        (Rendering|Material|SetScalarParameterValueonMaterials _button_handle "Brightness" 1e+01)
        (Transformation|SetRelativeLocation _button_handle (+ (Variables|/Script/Engine.SceneComponent|GetRelativeLocation _button_handle) "-10.000000,0.000000,0.000000") false false)
        (return _returnvalue))
      (:else))))